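; Player tool Blueprint for an actor settings menu, still unfinished.
; On the client it binds a custom action to C and caches the PlayerController; that action toggles an access flag and the mouse cursor.
; While toggled on, right-click runs a debug-drawn visibility trace from the deprojected cursor, but the hit is unused.
; The physgun settings event is empty, and the physics constraint code on a selected actor is unconnected.
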(event EventBeginPlay
  ;[1 1 1] Begin Play
  (|CallParentFunction)
  (Utilities|HandleClientServerLogic
    (:ClientLogic
      (Class|KJModToolProxy|SetCustomAction "C" "ActorSettings_Access" "Used for accessing the tool" 2) ; Used for enabling input
      (CallFunction|NotifyOwnerOfInstantiation) ; Initiate the tool
      (bind _ascharacter (Utilities|Casting|CastToCharacter (Components|GetOwner)))
      (bind _asplayer_controller (Utilities|Casting|CastToPlayerController (Pawn|GetController _ascharacter)))
      (Variables|Default|SetPlayerController _asplayer_controller) ; Get PlayerController Reference
    )))

(event EventTick
  (params (DeltaSeconds :type Float%20%28single-precision%29))
  (|CallParentFunction DeltaSeconds))

(event EventToolProxyCustomActionPressed
  (params (cookie :type Integer) (pressed :type Boolean))
  (bind _playercontroller (Variables|Default|GetPlayerController))
  (if (== cookie 2)
    (if pressed
      (if (Variables|Default|GetbPressingInputKey?)
        (Variables|Default|SetbPressingInputKey? false)
        (Variables|/Script/Engine.PlayerController|SetbShowMouseCursor _playercontroller false)
        (else
          (Variables|Default|SetbPressingInputKey? true)
          (Variables|/Script/Engine.PlayerController|SetbShowMouseCursor _playercontroller true))))))

(event EventToolProxySecondaryMouseClick
  (params (pressed :type Boolean))
  (bind _playercontroller (Variables|Default|GetPlayerController))
  (bind (_worldlocation _worlddirection) (Game|Player|ConvertMouseLocationToWorldSpace _playercontroller))
  (if pressed
    (Development|PrintString "RIGHT CLICK PRESSED")
    (if (Variables|Default|GetbPressingInputKey?)
      (Collision|LineTraceByChannel _worldlocation (* _worlddirection (+ (Math|Vector|GetForwardVector (Pawn|GetControlRotation _playercontroller :!class /Script/Engine.Controller)) 5e+03)) "TraceTypeQuery1" false 0 "Persistent")
      (Development|PrintString "LINE TRACED")
      (else
        (Development|PrintString "NOT PRESSING INPUT KEY")))))

(event Custom|ChangePhysgunSettings)

(fn ConstructionScript
  (|CallParentFunction))