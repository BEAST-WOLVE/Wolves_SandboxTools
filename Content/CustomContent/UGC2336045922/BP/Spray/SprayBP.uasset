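; SprayBP is a spray actor that shows an image downloaded from a URL on a decal.
; Clients create a dynamic material instance showing a loading texture, then swap in the downloaded image, or an error texture on failure or empty URL.
; Setting changes pass through a retriggerable delay to a server event and multicast that refreshes the image.
; Replicated settings also apply decal rotation and optional attachment, destroying the spray with its parent.
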(event Custom|OC_ChangeSettings
  (params (Settings :type Spray%20Settings%20Struct%20Structure))
  ;[1 1 1] Change Settings
  (Utilities|FlowControl|RetriggerableDelay 0.1) ; Spam Protection
  (CallFunction|SChangeSettings Settings))

(event Custom|MC_ChangeSettings
  (params (Settings :type Spray%20Settings%20Struct%20Structure))
  ;[1 1 1] Change Settings
  (Utilities|HandleClientServerLogic ; Only on Client -> Server has no Visuals
    (:ClientLogic
      (Variables|Default|SetSettings Settings)
      (CallFunction|OCSetImage))))

(event Custom|OC_SetImage
  (bind _decal (Variables|Default|GetDecal))
  (bind _settings (Variables|Default|GetSettings))
  (bind _img_url (Utilities|Struct|BreakSpraySettingsStruct _settings))
  ;[1 1 1] Set Image on each Client
  (if (Utilities|Enum|NotEqual(Enum) _img_url "")
    (bind _texture (|DownloadImage _img_url) ; Download Image from the Internet
      (:then
        (Rendering|Components|Decal|SetDecalMaterial _decal "/Game/CustomContent/UGC2336045922/Assets/MI_Spray.MI_Spray")
        (bind _returnvalue (Rendering|Material|CreateDynamicMaterialInstance _decal :!class /Script/Engine.DecalComponent))
        (bind _output_get (Variables|Default|SetLocalMatInstance _returnvalue))
        (Rendering|Material|SetTextureParameterValue _output_get "IMG" "/Game/CustomContent/UGC2336045922/Assets/T_Loading.T_Loading") ; Created a dynamic instance and set it's image to "Loading", while downloading
      )
      (:OnSuccess
        (Utilities|FlowControl|Delay 0.1) ; If internet is too fast, wait to debug
        (Rendering|Material|SetTextureParameterValue (Variables|Default|GetLocalMatInstance) "IMG" _texture) ; On Success, apply Image
      )
      (:OnFail
        (Rendering|Material|SetTextureParameterValue (Variables|Default|GetLocalMatInstance) "IMG" "/Game/CustomContent/UGC2336045922/Assets/T_Bad.T_Bad" :!label _label) ; On Fail or Input was empty, use "Bad" Image, to indicate fail
      ))
    (else
      (goto _label))))

(event Custom|S_ChangeSettings
  (params (Settings :type Spray%20Settings%20Struct%20Structure))
  ;[1 1 1] Change Settings
  (CallFunction|MCChangeSettings Settings))

(event Custom|RealiseRotation
  (params (Rotation :type Float%20%28single-precision%29))
  ;[1 1 1] Rotation
  (Transformation|SetRelativeRotation (Variables|Default|GetDecal) (Math|Rotator|MakeRotator Rotation 0.0 0.0) false false))

(event Custom|RealiseSettings
  (params (Settings :type Spray%20Settings%20Struct%20Structure))
  (bind (_img_url _attach_ _attachto _rotation) (Utilities|Struct|BreakSpraySettingsStruct Settings))
  ;[1 1 1] Apply Final Settings
  (Utilities|HandleClientServerLogic
    (:ServerLogic
      _)
    (:ClientLogic
      (CallFunction|OCSetImage)
      (CallFunction|RealiseRotation _rotation)))
  (if _attach_
    (Transformation|AttachActorToActor _attachto "None" "KeepWorld" "KeepWorld" "KeepWorld" true)
    (Game|BindEventtoOnDestroyed _attachto (delegate Custom|AttachParentDestroyed))))

(event Custom|AttachParentDestroyed
  (params (DestroyedActor :type Actor%20Object%20Reference))
  ;[1 1 1] Apply Final Settings
  (Actor|DestroyActor))

(event EventBeginPlay
  ;[1 1 1] SetImage on Begin Play
  (Utilities|HandleClientServerLogic
    (:ClientLogic
      (CallFunction|OCSetImage))))

(fn ConstructionScript)

(fn OnRepSettings
  (CallFunction|RealiseSettings (Variables|Default|GetSettings)))