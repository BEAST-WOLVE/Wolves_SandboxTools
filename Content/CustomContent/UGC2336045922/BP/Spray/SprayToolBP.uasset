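; Player tool that places image sprays (SprayBP) on surfaces the camera points at.
; The local client traces each tick to move a ghost preview, itself the first spawned SprayBP, and relays its transform to the server.
; Left click spawns a spray that gets the current settings and attaches to the hit component, right click rotates, wheel scales.
; Image URL and attach settings come from a save or settings widget; OnRep records sprays in removal history.
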(event Custom|AdjustGhostSpraySettings
  (params (Settings :type Spray%20Settings%20Struct%20Structure))
  ;[1 1 1] Ghost Spray - Change
  (Utilities|IsValid (Variables|Ghosting|GetGhostSpray)
    (:Is%20Valid
      (Default|OCChangeSettings (Variables|Ghosting|GetGhostSpray) Settings))))

(event Custom|UpdateHistoryOwningClient
  (params (ObjectToAttach :type Actor%20Object%20Reference))
  ;[1 1 1] Update the history (to reflect last selection as most recent)
  (Class|KJModToolProxy|AddHistoryEntry (Utilities|Struct|MakeKJModToolHistoryItem ObjectToAttach "Removing spray" "Spray" "DeleteItem")))

(event Custom|SetGhostSprayInformationOwningClient
  (params (IsVisible :type Boolean) (Location :type Vector) (Rotation :type Rotator) (Scale :type Vector))
  (bind _ghostspray (Variables|Ghosting|GetGhostSpray))
  ;[1 1 1] Ghost Spray Update - Update spray position and settings information (local and remote)
  (CallFunction|SetGhostSprayInformationServer IsVisible Location Rotation Scale)
  (Utilities|IsValid _ghostspray ; may not be replicated yet
    (:Is%20Valid
      (Transformation|SetActorLocation _ghostspray Location false true)
      (Transformation|SetActorRotation _ghostspray Rotation true)
      (Transformation|SetActorScale3D _ghostspray Scale)
      (Rendering|SetActorHiddenInGame _ghostspray (not IsVisible)))))

(event Custom|SetGhostSprayInformationServer
  (params (Visible :type Boolean) (Location :type Vector) (Rotation :type Rotator) (Scale :type Vector))
  (bind _ghostspray (Variables|Ghosting|GetGhostSpray))
  ;[1 1 1] Ghost Spray Update - Update spray position and settings information (local and remote)
  (Utilities|IsValid _ghostspray ; Is null when switching lamp's
    (:Is%20Valid
      (Transformation|SetActorLocation _ghostspray Location false true)
      (Transformation|SetActorRotation _ghostspray Rotation true)
      (Transformation|SetActorScale3D _ghostspray Scale))))

(event EventDestroyed
  (bind _ghostspray (Variables|Ghosting|GetGhostSpray))
  ;[1 1 1] DESTROYED - remove ghost spray from server
  (Utilities|IsValid _ghostspray
    (:Is%20Valid
      (Actor|DestroyActor _ghostspray))))

(event EventBeginPlay
  ;[0.9593 1 0.1335] BEGIN PLAY EVENT
  (Utilities|HandleClientServerLogic
    (:ClientLogic
      (Class|KJModToolProxy|SetCustomAction "C" "Spray_Scale" "Used for scaling sprays" 1)
      ;;[1 1 1] If local controlled; init once..
      (Utilities|IsLocallyControlled
        (:LocalControl
          (CallFunction|NotifyOwnerOfInstantiation)
          (if (not (Variables|Initialisation|GetInitialised))
            (Variables|Initialisation|SetInitialised true)
            ;;[1 1 1] Reload settings
            (CallFunction|CreateandShowToolsAssistInformation)
            (CallFunction|InitSettings)
            ;;[1 1 1] Create ghost text
            (CallFunction|CreateGhostSpray)))))))

(event EventTick
  (params (DeltaSeconds :type Float%20%28single-precision%29))
  ;[1 1 1] EVENT TICK
  (|CallParentFunction DeltaSeconds)
  (Utilities|IsLocallyControlled
    (:LocalControl
      (Utilities|HandleClientServerLogic
        (:ClientLogic
          ;;[1 1 1] Handle MOUSE SELECTION POINT
          (bind _returnvalue (Class|KJModToolProxy|GetPawnCameraComponent))
          (bind (_outhit _returnvalue_2) (Collision|LineTraceByChannel (Transformation|GetWorldLocation _returnvalue) (+ (Transformation|GetWorldLocation _returnvalue) (* (Math|Vector|GetForwardVector _returnvalue) 1.5e+03)) "TraceTypeQuery1" true (Utilities|Array|MakeArray (Game|Player|GetPlayerPawn 0) (Variables|Ghosting|GetGhostSpray)) "ForDuration" true "(R=1.000000,G=0.000000,B=0.000000,A=1.000000)" "(R=0.000000,G=1.000000,B=0.000000,A=1.000000)" 1.0))
          (if _returnvalue_2
            (Utilities|IsValid (.HitActor (Collision|BreakHitResult _outhit))
              (:Is%20Valid
                (Utilities|IsValid (Variables|Ghosting|GetGhostSpray) ; May not be replicated from server (yet)
                  (:Is%20Valid
                    (bind _structout (Utilities|Struct|SetmembersinSpraySettingsStruct (Variables|ToolSetting|GetRunTimeSettings) (.HitActor (Collision|BreakHitResult _outhit))))
                    (Variables|ToolSetting|SetRunTimeSettings _structout)
                    (bind _rotation (Utilities|BuildRotationfromImpactNormal (.ImpactPoint (Collision|BreakHitResult _outhit)) (.ImpactNormal (Collision|BreakHitResult _outhit)))
                      (:Out
                        (Variables|Ghosting|SetGhostSprayLocation (.ImpactPoint (Collision|BreakHitResult _outhit)))
                        (Variables|Ghosting|SetGhostSprayRotation _rotation)
                        (Variables|Spawning|SetAttachToComponent (.HitComponent (Collision|BreakHitResult _outhit)))
                        (CallFunction|SetGhostSprayInformationOwningClient true (Variables|Ghosting|GetGhostSprayLocation) (Variables|Ghosting|GetGhostSprayRotation) (Variables|Ghosting|GetGhostSprayScale))
                        (Variables|Ghosting|SetGhostSprayVisible true))))
                  (:Is%20Not%20Valid
                    (CallFunction|SetGhostSprayInformationOwningClient false "0, 0, 0" "0, 0, 0" "0, 0, 0" :!label _label)
                    (Variables|Ghosting|SetGhostSprayVisible false))))
              (:Is%20Not%20Valid
                (goto _label)))
            (else
              (goto _label))))))))

(event Custom|ServerReleaseSpray
  (params (SprayToRelease :type Spray%20BP%20Object%20Reference))
  ;[1 1 1] SERVER - Release Spray; we need to set it's settings so they are set (and it visualises itself correctly) + Attach it to the it component
  (Variables|/Game/CustomContent/UGC2336045922/BP/Spray/SprayBP.SprayBP_C|SetSettings SprayToRelease (Variables|ToolSetting|GetRunTimeSettings))
  (Transformation|AttachComponentToComponent SprayToRelease (Variables|Spawning|GetAttachToComponent) "None" "KeepWorld" "KeepWorld" "KeepWorld" true))

(event EventToolProxyItemSpawned
  (params (spawnedActor :type Actor%20Object%20Reference))
  ;[1 1 1] (interface) Item Spawned - From Pawn
  (bind _asspray_bp (Utilities|Casting|CastToSprayBP spawnedActor)
    (:then
      (Utilities|IsValid (Variables|Ghosting|GetGhostSpray) ; First time? it's our "ghost" spray
        (:Is%20Valid
          (bind _output_get (Variables|Spawning|SetSpawnedSprayActor _asspray_bp))
          (CallFunction|ServerReleaseSpray _output_get))
        (:Is%20Not%20Valid
          (Variables|Ghosting|SetGhostSpray _asspray_bp)
          (CallFunction|AdjustGhostSpraySettings (Variables|ToolSetting|GetRunTimeSettings)))))
    (:CastFailed
      (|CallParentFunction spawnedActor) ; Probably a Q menu spawning; let parent deal with it
    )))

(event EventToolProxySecondaryMouseClick
  (params (pressed :type Boolean))
  ;[1 1 1] RIGHT - Change Rotation
  (if pressed
    (Utilities|IsValid (Variables|Ghosting|GetGhostSpray)
      (:Is%20Valid
        (if (Variables|Ghosting|GetGhostSprayVisible)
          (bind _output_get (Variables|Default|SetAdditionalXRotation (+ (Variables|Default|GetAdditionalXRotation) 9e+01)))
          (bind _structout (Utilities|Struct|SetmembersinSpraySettingsStruct (Variables|ToolSetting|GetRunTimeSettings) _output_get))
          (Default|RealiseRotation (Variables|Ghosting|GetGhostSpray) (.Rotation (Utilities|Struct|BreakSpraySettingsStruct _structout))))))))

(event EventToolProxyPrimaryMouseClick
  (params (pressed :type Boolean))
  ;[1 1 1] Left - Attempt Spray
  (if pressed
    (Utilities|IsValid (Variables|Ghosting|GetGhostSpray)
      (:Is%20Valid
        (if (Variables|Ghosting|GetGhostSprayVisible)
          (Class|KJModToolProxy|SpawnItem "/Game/CustomContent/UGC2336045922/BP/Spray/SprayBP" (Variables|Ghosting|GetGhostSprayLocation) (Variables|Ghosting|GetGhostSprayRotation) (Variables|Ghosting|GetGhostSprayScale))
          (Class|KJModToolProxy|PlayToolSoundEffect "ToolSpawnSound" true))))))

(event EventToolProxyMouseWheelAxisChanged
  (params (axisDelta :type Float%20%28single-precision%29))
  ;[1 1 1] WHEEL - Scale Spray
  (Utilities|IsValid (Variables|Ghosting|GetGhostSpray)
    (:Is%20Valid
      (if (> axisDelta 0.0)
        (if (< (.X (Math|Vector|BreakVector (Variables|Ghosting|GetGhostSprayScale))) 3.0)
          (bind _output_get (Variables|Ghosting|SetGhostSprayScale (+ (Variables|Ghosting|GetGhostSprayScale) 0.1)))
          (CallFunction|SetGhostSprayInformationOwningClient (Variables|Ghosting|GetGhostSprayVisible) (Variables|Ghosting|GetGhostSprayLocation) (Variables|Ghosting|GetGhostSprayRotation) _output_get))
        (elif (< axisDelta 0.0)
          (if (> (.X (Math|Vector|BreakVector (Variables|Ghosting|GetGhostSprayScale))) 0.1)
            (bind _output_get_2 (Variables|Ghosting|SetGhostSprayScale (+ (Variables|Ghosting|GetGhostSprayScale) -0.1)))
            (CallFunction|SetGhostSprayInformationOwningClient (Variables|Ghosting|GetGhostSprayVisible) (Variables|Ghosting|GetGhostSprayLocation) (Variables|Ghosting|GetGhostSprayRotation) _output_get_2)))))))

(event Custom|Settings_URLChanged
  (params (IMG_URL :type String))
  ;[1 1 1] Settings (from widgets and onload)
  (bind _structout (Utilities|Struct|SetmembersinSpraySettingsStruct (Variables|ToolSetting|GetRunTimeSettings) IMG_URL))
  (CallFunction|AdjustGhostSpraySettings _structout)
  ;[1 1 1] Update server
  (if (Variables|ToolSetting|GetbServerSettingsInited)
    (CallFunction|SetSpraySettingsOwningClient (Variables|ToolSetting|GetRunTimeSettings))))

(event Custom|Settings_AttachChanged
  (params (Attached :type Boolean))
  ;[1 1 1] Settings (from widgets and onload)
  (bind _structout (Utilities|Struct|SetmembersinSpraySettingsStruct (Variables|ToolSetting|GetRunTimeSettings) Attached))
  (CallFunction|AdjustGhostSpraySettings _structout)
  ;[1 1 1] Update server
  (if (Variables|ToolSetting|GetbServerSettingsInited)
    (CallFunction|SetSpraySettingsOwningClient (Variables|ToolSetting|GetRunTimeSettings))))

(event Custom|SetSpraySettingsOwningClient
  (params (Settings :type Spray%20Settings%20Struct%20Structure))
  ;[1 1 1] Replicate changes
  (CallFunction|SetSpraySettingsServer Settings))

(event Custom|SetSpraySettingsServer
  (params (Settings :type Spray%20Settings%20Struct%20Structure))
  ;[1 1 1] Replicate changes
  (Variables|ToolSetting|SetRunTimeSettings Settings))

(event Custom|InitSettings
  ;[1 1 1] Init / Load previous settings
  (bind _returnvalue (Class|KJModToolProxy|LoadToolSettings "SprayToolSettings_27Dec2020_2010"))
  (Utilities|IsValid _returnvalue ; No save? use defaults
    (:Is%20Valid
      (bind _asspray_tool_save_game_bp (Utilities|Casting|CastToSprayToolSaveGameBP _returnvalue))
      (Utilities|FlowControl|Sequence
        (:then_0
          ;[1 1 1] Local Initial settings
          (CallFunction|SettingsURLChanged (Variables|/Game/CustomContent/UGC2336045922/BP/Spray/SprayToolSaveGameBP.SprayToolSaveGameBP_C|GetIMG_Link _asspray_tool_save_game_bp)))
        (:then_2
          (CallFunction|SettingsAttachChanged (Variables|/Game/CustomContent/UGC2336045922/BP/Spray/SprayToolSaveGameBP.SprayToolSaveGameBP_C|GetAttach? _asspray_tool_save_game_bp)))
        (:then_3
          ;;[1 1 1] Init settings server
          (CallFunction|SetSpraySettingsOwningClient (Variables|ToolSetting|GetRunTimeSettings) :!label _label)
          (Variables|ToolSetting|SetbServerSettingsInited true))))
    (:Is%20Not%20Valid
      (goto _label))))

(fn ConstructionScript)

(fn CreateandShowToolsAssistInformation
  (Class|KJModToolProxy|ShowToolAssistUI)
  (Class|KJModToolProxy|SetToolAssistTitle "Spray" "Sprays can display an image")
  (Class|KJModToolProxy|ClearToolAssistFunctions)
  (bind _returnvalue (Class|KJModToolProxy|CreateToolAssistFunction "Add spray to the selected point"))
  (Class|KJModToolProxy|SetToolAssistFunctionPrimaryDetails _returnvalue "LeftMouse"))

(fn CreateGhostSpray
  (bind _returnvalue (Game|GetPlayerCameraManager 0))
  (Class|KJModToolProxy|SpawnItem "/Game/CustomContent/UGC2336045922/BP/Spray/SprayBP" (+ (Transformation|GetActorLocation _returnvalue) (* (Transformation|GetActorForwardVector _returnvalue) 5e+02)) "0, 0, 0" "1.000000,1.000000,1.000000"))

(fn ToolProxyGetToolSettingPanel
  (Utilities|IsValid (Variables|ToolSetting|GetToolSettingsWidget)
    (:Is%20Valid
      _)
    (:Is%20Not%20Valid
      (bind _returnvalue (UserInterface|CreateWidget "/Game/CustomContent/UGC2336045922/BP/Spray/SpraySettings/SprayToolSettingsWidgetBP.SprayToolSettingsWidgetBP_C" (Game|GetPlayerController 0) self))
      (Default|CreatedEvent _returnvalue)
      (Variables|ToolSetting|SetToolSettingsWidget _returnvalue)))
  (return (Variables|ToolSetting|GetToolSettingsWidget)))

(fn OnRepSpawnedSprayActor
  (bind _spawnedsprayactor (Variables|Spawning|GetSpawnedSprayActor))
  ;[1 1 1] If we're the owner then record the text creation in our history (for delete)
  (Utilities|IsLocallyControlled
    (:LocalControl
      (Utilities|IsValid _spawnedsprayactor
        (:Is%20Valid
          (CallFunction|UpdateHistoryOwningClient _spawnedsprayactor))))))