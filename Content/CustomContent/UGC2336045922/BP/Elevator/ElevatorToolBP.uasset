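; Player tool that turns a prop into an elevator, with a settings panel and on-screen control hints.
; Tick traces from the camera and highlights props green, or red if static, simulating physics, already elevators or not owned.
; Left click toggles a ghost ElevatorProp with the prop attached, mouse wheel adjusts height or speed, and right click confirms and tags it.
; The wait interval loads from a save game, and settings pass to the server through OC/S events.
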(event Custom|UpdateHistoryOwningClient
  (params (ObjectToAttach :type Actor%20Object%20Reference))
  ;[1 1 1] Update the history (to reflect last selection as most recent)
  (Class|KJModToolProxy|AddHistoryEntry (Utilities|Struct|MakeKJModToolHistoryItem ObjectToAttach "elevator" "Elevator" "DeleteItem")))

(event EventDestroyed
  (bind _ghostelevator (Variables|Ghosting|GetGhostElevator))
  (bind _playercontroller (Variables|Default|GetPlayerController))
  ;[1 1 1] DESTROYED - remove selection marker
  (Utilities|IsValid _ghostelevator
    (:Is%20Valid
      (Actor|DestroyActor _ghostelevator)
      (Class|KJModUtilityActor|RemoveObjectHighlight _playercontroller (Variables|Default|GetLastHitActor))
      (Class|KJModUtilityActor|RemoveObjectHighlight _playercontroller (Variables|Targeting|GetSelectedActor)))))

(event EventBeginPlay
  ;[0.9593 1 0.1335] BEGIN PLAY EVENT
  (Utilities|HandleClientServerLogic
    (:ClientLogic
      ;;[1 1 1] Add CustomKeyInput
      (Class|KJModToolProxy|SetCustomAction "LeftShift" "Elevator_SlowAdjust" "Adjust the elevator height more exact" 1)
      (Class|KJModToolProxy|SetCustomAction "C" "Elevator_Speed" "Adjust the elevator height more exact" 2)
      ;;[1 1 1] If local controlled; init once..
      (CallFunction|NotifyOwnerOfInstantiation)
      (if (not (Variables|Initialisation|GetInitialised))
        (Variables|Initialisation|SetInitialised true)
        ;;[1 1 1] Reload settings
        (CallFunction|CreateandShowToolsAssistInformation)
        (CallFunction|InitSettings)
        ;;[1 1 1] Get PlaerController from Owner
        (bind _ascharacter (Utilities|Casting|CastToCharacter (Components|GetOwner)))
        (bind _asplayer_controller (Utilities|Casting|CastToPlayerController (Pawn|GetController _ascharacter)))
        (Variables|Default|SetPlayerController _asplayer_controller) ; Get PlayerController Reference
      ))))

(event EventTick
  (params (DeltaSeconds :type Float%20%28single-precision%29))
  ;[1 1 1] EVENT TICK
  (|CallParentFunction DeltaSeconds)
  (if (not (Variables|Default|GetActorSelected?)) ; Only execute, if there is no selection
    (Utilities|IsLocallyControlled
      (:LocalControl
        (Networking|SwitchHasAuthority
          (:Authority
            ;;[1 1 1] Listen server?
            (if (not (Networking|IsDedicatedServer))
              ;;[1 1 1] Handle Selection
              (bind _returnvalue (Class|KJModToolProxy|GetPawnCameraComponent :!label _label))
              (bind (_outhit _returnvalue_2) (Collision|LineTraceByChannel (Transformation|GetWorldLocation _returnvalue) (+ (Transformation|GetWorldLocation _returnvalue) (* (Math|Vector|GetForwardVector _returnvalue) 3.5e+03)) "TraceTypeQuery1" true (Utilities|Array|MakeArray (Game|Player|GetPlayerPawn 0)) "None"))
              (Utilities|FlowControl|Sequence
                (:then_0
                  (if _returnvalue_2
                    (Utilities|IsValid (.HitActor (Collision|BreakHitResult _outhit))
                      (:Is%20Valid
                        (bind _bhaslocalownership (Class|KJModOwnershipComponent|HasOwnershipRights 0 true (Utilities|GetSteamUserID) (.HitActor (Collision|BreakHitResult _outhit))))
                        (if (Math|Boolean|ORBoolean (or (Utilities|Enum|Equal(Enum) (Variables|/Script/Engine.SceneComponent|GetMobility (.HitComponent (Collision|BreakHitResult _outhit))) "Static") (Utilities|Enum|Equal(Enum) (Variables|/Script/Engine.SceneComponent|GetMobility (.HitComponent (Collision|BreakHitResult _outhit))) "Stationary")) (Physics|IsSimulatingPhysics (.HitComponent (Collision|BreakHitResult _outhit)) "None") (Actor|ActorHasTag (.HitActor (Collision|BreakHitResult _outhit)) "Elevator") (not _bhaslocalownership)) ; Check for many conditions...
                          (Class|KJModUtilityActor|AddObjectHighlight (Variables|Default|GetPlayerController) (.HitActor (Collision|BreakHitResult _outhit)) "Red")
                          (Variables|Targeting|SetSelectedActor (.HitActor (Collision|BreakHitResult _outhit)))
                          (bind _structout (Utilities|Struct|SetmembersinElevatorToolActorSettings (Utilities|Struct|MakeElevatorToolActorSettings)))
                          (Variables|ToolSetting|SetSettings _structout)
                          (else
                            (Class|KJModUtilityActor|AddObjectHighlight (Variables|Default|GetPlayerController) (.HitActor (Collision|BreakHitResult _outhit)) "Green")
                            (Variables|Targeting|SetSelectedActor (.HitActor (Collision|BreakHitResult _outhit)))
                            (bind _structout_2 (Utilities|Struct|SetmembersinElevatorToolActorSettings (Utilities|Struct|MakeElevatorToolActorSettings (.HitActor (Collision|BreakHitResult _outhit)))))
                            (Variables|ToolSetting|SetSettings _structout_2)))))))
                (:then_1
                  (if (not (== (.HitActor (Collision|BreakHitResult _outhit)) (Variables|Default|GetLastHitActor)))
                    (if (!= (Variables|Default|GetLastHitActor) (Variables|Targeting|GetSelectedActor))
                      (Class|KJModUtilityActor|RemoveObjectHighlight (Game|GetPlayerController 0) (Variables|Default|GetLastHitActor))
                      (Variables|Default|SetLastHitActor (.HitActor (Collision|BreakHitResult _outhit)))))))))
          (:Remote
            (goto _label)))))))

(event Custom|S_SetNewHeight
  (params (AddNewHeight :type Float%20%28single-precision%29))
  ;[1 1 1] CHANGE HEIGHT
  (if (Math|Float|InRange(Float) (+ AddNewHeight (Utilities|Struct|BreakElevatorToolActorSettings (Variables|ToolSetting|GetSettings))) 1e+02 5e+03)
    (Utilities|Struct|SetmembersinElevatorToolActorSettings (Variables|ToolSetting|GetSettings) (+ AddNewHeight (Utilities|Struct|BreakElevatorToolActorSettings (Variables|ToolSetting|GetSettings))))
    (Transformation|AddRelativeLocation (Variables|/Game/CustomContent/UGC2336045922/BP/Elevator/Prop/ElevatorProp.ElevatorProp_C|GetMaxHeightRoot (Variables|Ghosting|GetGhostElevator)) (Math|Vector|MakeVector 0.0 0.0 AddNewHeight) false false)))

(event Custom|S_SetNewSpeed
  (params (AddNewSpeed :type Float%20%28single-precision%29))
  (bind _settings (Variables|ToolSetting|GetSettings))
  (bind _elevatorspeed (Utilities|Struct|BreakElevatorToolActorSettings _settings))
  (bind _returnvalue (+ AddNewSpeed _elevatorspeed))
  ;[1 1 1] CHANGE SPEED
  (if (and (> _returnvalue 1.0) (< _returnvalue 6e+01))
    (bind _structout (Utilities|Struct|SetmembersinElevatorToolActorSettings (Variables|ToolSetting|GetSettings) (+ AddNewSpeed (Utilities|Struct|BreakElevatorToolActorSettings (Variables|ToolSetting|GetSettings)))))
    (Default|SChangeSettings (Variables|Ghosting|GetGhostElevator) _structout)))

(event EventToolProxySecondaryMouseClick
  (params (pressed :type Boolean))
  (bind _settings (Variables|ToolSetting|GetSettings))
  (bind (_elevatorspeed _elevatorwaitinterval) (Utilities|Struct|BreakElevatorToolActorSettings _settings))
  ;[1 1 1] RIGHT MOUSE - Confirm Elevator
  (if pressed
    (Utilities|IsValid (Utilities|Struct|BreakElevatorToolActorSettings (Variables|ToolSetting|GetSettings))
      (:Is%20Valid
        (if (Variables|Default|GetActorSelected?)
          (Default|SRealiseSettings (Variables|Ghosting|GetGhostElevator) (Utilities|Struct|MakeElevatorToolActorSettings _elevatorspeed _elevatorwaitinterval (Variables|Targeting|GetSelectedActor)))
          (Class|KJModUtilityActor|RemoveObjectHighlight (Variables|Default|GetPlayerController) (Variables|Targeting|GetSelectedActor))
          (Class|KJModToolProxy|PlayToolSoundEffect "ToolSelectionSound" true)
          (Utilities|Array|Add (Variables|/Script/Engine.Actor|GetTags (Variables|Targeting|GetSelectedActor)) "Elevator") ; Get ignored by elevator tool
          (Utilities|Array|Add (Variables|/Script/Engine.Actor|GetTags (Variables|Targeting|GetSelectedActor)) "IgnorePhysgun") ; Disable moving
          (Variables|Default|SetActorSelected? false)
          (Variables|Targeting|SetSelectedActor 0)
          (Variables|Ghosting|SetGhostElevator 0)
          (Class|KJModToolProxy|PlayToolSoundEffect "ToolSpawnSound" true))))))

(event EventToolProxyCustomActionPressed
  (params (cookie :type Integer) (pressed :type Boolean))
  ;[1 1 1] CUSTOM KEY
  (if (== cookie 1)
    (if pressed
      (Variables|Default|SetSmoothAdjust? true)
      (else
        (Variables|Default|SetSmoothAdjust? false)))
    (elif (== cookie 2)
      (if pressed
        (Variables|Default|SetAdjustSpeed? true)
        (else
          (Variables|Default|SetAdjustSpeed? false))))))

(event EventToolProxyPrimaryMouseClick
  (params (pressed :type Boolean))
  ;[1 1 1] LEFT MOUSE - Select Prop as Elevator
  (if pressed ; Pressed?
    (Utilities|IsValid (Utilities|Struct|BreakElevatorToolActorSettings (Variables|ToolSetting|GetSettings))
      (:Is%20Valid
        (if (Variables|Default|GetActorSelected?)
          (Variables|/Game/CustomContent/UGC2336045922/BP/Elevator/Prop/ElevatorProp.ElevatorProp_C|SetWasUndo? (stale _returnvalue) true)
          (Actor|DestroyActor (stale _returnvalue))
          (Variables|Default|SetActorSelected? false)
          (Variables|Targeting|SetSelectedActor 0)
          (else
            (Variables|Default|SetActorSelected? true)
            (Class|KJModUtilityActor|AddObjectHighlight (Variables|Default|GetPlayerController) (Variables|Targeting|GetSelectedActor) "Blue")
            (bind _returnvalue (Game|SpawnActorfromClass "/Game/CustomContent/UGC2336045922/BP/Elevator/Prop/ElevatorProp.ElevatorProp_C" (Math|Transform|MakeTransform (Transformation|GetWorldLocation (Variables|/Script/Engine.Actor|GetRootComponent (Variables|Targeting|GetSelectedActor))) "0, 0, 0" (Transformation|GetWorldScale (Variables|/Script/Engine.Actor|GetRootComponent (Variables|Targeting|GetSelectedActor)))) "Undefined" 0 0))
            (Variables|Ghosting|SetGhostElevator _returnvalue)
            (Actor|SetOwner (Variables|Ghosting|GetGhostElevator) (Components|GetOwner))
            (Transformation|AttachComponentToComponent (Variables|Targeting|GetSelectedActor) (Variables|/Game/CustomContent/UGC2336045922/BP/Elevator/Prop/ElevatorProp.ElevatorProp_C|GetElevatorParent (Variables|Ghosting|GetGhostElevator)) "None" "KeepWorld" "KeepWorld" "KeepWorld" true)
            (Transformation|SetRelativeLocation (Variables|/Game/CustomContent/UGC2336045922/BP/Elevator/Prop/ElevatorProp.ElevatorProp_C|GetElevatorPreview (Variables|Ghosting|GetGhostElevator)) (Math|Vector|MakeVector (.x (Math|Transform|InverseTransformLocation (Math|Transform|MakeTransform (.location (Transformation|GetWorldTransform (Variables|/Game/CustomContent/UGC2336045922/BP/Elevator/Prop/ElevatorProp.ElevatorProp_C|GetMaximumHeight (Variables|Ghosting|GetGhostElevator)))) "0, 0, 0" "1,1,1") (.Origin (Collision|GetComponentBounds (Actor|GetComponentbyClass (Variables|Targeting|GetSelectedActor) "/Script/Engine.StaticMeshComponent"))))) (.y (Math|Transform|InverseTransformLocation (Math|Transform|MakeTransform (.location (Transformation|GetWorldTransform (Variables|/Game/CustomContent/UGC2336045922/BP/Elevator/Prop/ElevatorProp.ElevatorProp_C|GetMaximumHeight (Variables|Ghosting|GetGhostElevator)))) "0, 0, 0" "1,1,1") (.Origin (Collision|GetComponentBounds (Actor|GetComponentbyClass (Variables|Targeting|GetSelectedActor) "/Script/Engine.StaticMeshComponent"))))) (.z (Math|Transform|InverseTransformLocation (Math|Transform|MakeTransform (.location (Transformation|GetWorldTransform (Variables|/Game/CustomContent/UGC2336045922/BP/Elevator/Prop/ElevatorProp.ElevatorProp_C|GetMaximumHeight (Variables|Ghosting|GetGhostElevator)))) "0, 0, 0" "1,1,1") (.Origin (Collision|GetComponentBounds (Actor|GetComponentbyClass (Variables|Targeting|GetSelectedActor) "/Script/Engine.StaticMeshComponent")))))) false false) ; Set Location to match object in 3D Space
            (Transformation|SetWorldScale3D (Variables|/Game/CustomContent/UGC2336045922/BP/Elevator/Prop/ElevatorProp.ElevatorProp_C|GetMaximumHeight (Variables|Ghosting|GetGhostElevator)) (.BoxExtent (Collision|GetComponentBounds (Actor|GetComponentbyClass (Variables|Targeting|GetSelectedActor) "/Script/Engine.StaticMeshComponent")))) ; Set Bounds Scale
            (Variables|/Game/CustomContent/UGC2336045922/BP/Elevator/Prop/ElevatorProp.ElevatorProp_C|SetSettings (Variables|Ghosting|GetGhostElevator) (Variables|ToolSetting|GetSettings))
            (Default|SSetLocation (Variables|Ghosting|GetGhostElevator))
            (Class|KJModToolProxy|PlayToolSoundEffect "ToolSelectionSound" true)))))))

(event EventToolProxyMouseWheelAxisChanged
  (params (axisDelta :type Float%20%28single-precision%29))
  ;[1 1 1] MOUSE WHEEL
  (if (> axisDelta 0.0)
    (if (not (Variables|Default|GetAdjustSpeed?))
      (if (Variables|Default|GetSmoothAdjust?)
        (CallFunction|SSetNewHeight 1e+01)
        (else
          (CallFunction|SSetNewHeight 5e+01)))
      (else
        (CallFunction|SSetNewSpeed 1.0)))
    (elif (< axisDelta 0.0)
      (if (not (Variables|Default|GetAdjustSpeed?))
        (if (Variables|Default|GetSmoothAdjust?)
          (CallFunction|SSetNewHeight -1e+01)
          (else
            (CallFunction|SSetNewHeight -5e+01)))
        (else
          (CallFunction|SSetNewSpeed -1.0))))))

(event Custom|Settings_ElevatorDelay
  (params (Interval :type Float%20%28single-precision%29))
  (bind _ghostelevator (Variables|Ghosting|GetGhostElevator))
  ;[1 1 1] Settings (from widgets and onload)
  (bind _structout (Utilities|Struct|SetmembersinElevatorToolActorSettings (Variables|ToolSetting|GetSettings) Interval))
  (Utilities|IsValid _ghostelevator
    (:Is%20Valid
      (Default|SChangeSettings _ghostelevator _structout)
      ;[1 1 1] Update server
      (if (Variables|ToolSetting|GetbServerSettingsInited)
        (CallFunction|OCSetElevatorSettings (Variables|ToolSetting|GetSettings))))))

(event Custom|OC_SetElevatorSettings
  (params (Settings :type Elevator%20Tool%20Actor%20Settings%20Structure))
  ;[1 1 1] Replicate changes
  (CallFunction|SSetElevatorSettings Settings))

(event Custom|S_SetElevatorSettings
  (params (Settings :type Elevator%20Tool%20Actor%20Settings%20Structure))
  (bind _ghostelevator (Variables|Ghosting|GetGhostElevator))
  ;[1 1 1] Replicate changes
  (bind _output_get (Variables|ToolSetting|SetSettings Settings))
  (Utilities|IsValid _ghostelevator
    (:Is%20Valid
      (Default|SChangeSettings _ghostelevator _output_get))))

(event Custom|InitSettings
  ;[1 1 1] Init / Load previous settings
  (bind _returnvalue (Class|KJModToolProxy|LoadToolSettings "ElevatorToolSettings"))
  (Utilities|IsValid _returnvalue ; No save? use defaults
    (:Is%20Valid
      (bind _aselevator_tool_save_game_bp (Utilities|Casting|CastToElevatorToolSaveGameBP _returnvalue))
      (Utilities|FlowControl|Sequence
        (:then_0
          ;[1 1 1] Local Initial settings
          (CallFunction|SettingsElevatorDelay (Variables|/Game/CustomContent/UGC2336045922/BP/Elevator/ElevatorToolSaveGameBP.ElevatorToolSaveGameBP_C|GetWaitInterval _aselevator_tool_save_game_bp)))
        (:then_1
          ;[1 1 1] Init settings server
          (CallFunction|OCSetElevatorSettings (Variables|ToolSetting|GetSettings) :!label _label)
          (Variables|ToolSetting|SetbServerSettingsInited true))))
    (:Is%20Not%20Valid
      (goto _label))))

(fn ConstructionScript)

(fn CreateandShowToolsAssistInformation
  (Class|KJModToolProxy|ShowToolAssistUI)
  (Class|KJModToolProxy|SetToolAssistTitle "Elevator" "Turn any prop into an elevator!")
  (Class|KJModToolProxy|ClearToolAssistFunctions)
  (bind _returnvalue (Class|KJModToolProxy|CreateToolAssistFunction "Select prop as elevator"))
  (Class|KJModToolProxy|SetToolAssistFunctionPrimaryDetails _returnvalue "LeftMouse")
  (bind _returnvalue_2 (Class|KJModToolProxy|CreateToolAssistFunction "Confirm prop"))
  (Class|KJModToolProxy|SetToolAssistFunctionPrimaryDetails _returnvalue_2 "RightMouse")
  (bind _returnvalue_3 (Class|KJModToolProxy|CreateToolAssistFunction "Change Elevator Height"))
  (Class|KJModToolProxy|SetToolAssistFunctionPrimaryDetails _returnvalue_3 "MouseWheelAxis")
  (bind _returnvalue_4 (Class|KJModToolProxy|CreateToolAssistFunction "Smooth Adjust Elevator Height"))
  (Class|KJModToolProxy|SetToolAssistFunctionPrimaryDetails _returnvalue_4 "MouseWheelAxis" "Shift")
  (bind _returnvalue_5 (Class|KJModToolProxy|CreateToolAssistFunction "Adjust Elevator Speed (in Seconds)"))
  (Class|KJModToolProxy|SetToolAssistFunctionPrimaryDetails _returnvalue_5 "MouseWheelAxis" "C"))

(fn ToolProxyGetToolSettingPanel
  (Utilities|IsValid (Variables|ToolSetting|GetToolSettingsWidget)
    (:Is%20Valid
      _)
    (:Is%20Not%20Valid
      (bind _returnvalue (UserInterface|CreateWidget "/Game/CustomContent/UGC2336045922/BP/Elevator/Settings/ElevatorToolSettingsWidgetBP.ElevatorToolSettingsWidgetBP_C" (Game|GetPlayerController 0) self))
      (Default|CreatedEvent _returnvalue)
      (Variables|ToolSetting|SetToolSettingsWidget _returnvalue)))
  (return (Variables|ToolSetting|GetToolSettingsWidget)))