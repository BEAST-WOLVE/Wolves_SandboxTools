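; Player tool that precisely nudges actors, pushing or pulling them along the aimed surface's normal by a configurable step.
; A per-tick camera trace validates targets (mobility, physics, moving-platform tag), highlighting them green or red.
; Left and right clicks move the selection through a server event and multicast, with optional sound.
; F toggles a WorldAxisBoundsActor for world-axis movement, locking the selected actor; settings load from a save game.
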(event EventDestroyed
  (bind _worldaxisactor (Variables|Default|GetWorldAxisActor))
  (bind _playercontroller (Variables|Default|GetPlayerController))
  ;[1 1 1] DESTROYED - remove selection marker
  (Class|KJModUtilityActor|RemoveObjectHighlight _playercontroller (Variables|Default|GetLastHitActor))
  (Class|KJModUtilityActor|RemoveObjectHighlight _playercontroller (Utilities|Struct|BreakPrecisionSelection (Variables|Targeting|GetSelection)))
  (Utilities|IsValid _worldaxisactor
    (:Is%20Valid
      (Actor|DestroyActor _worldaxisactor))))

(event EventBeginPlay
  ;[0.9593 1 0.1335] BEGIN PLAY EVENT
  (Utilities|HandleClientServerLogic
    (:ClientLogic
      ;;[1 1 1] Add CustomKeyInput
      (Class|KJModToolProxy|SetCustomAction "F" "Precision_WorldAxis" "Used for moving along world axis" 1)
      ;;[1 1 1] If local controlled; init once..
      (CallFunction|NotifyOwnerOfInstantiation)
      (if (not (Variables|Initialisation|GetInitialised))
        (Variables|Initialisation|SetInitialised true)
        ;;[1 1 1] Reload settings
        (CallFunction|CreateandShowToolsAssistInformation)
        (CallFunction|InitSettings)
        ;;[1 1 1] Get PlayerController from Owner
        (bind _ascharacter (Utilities|Casting|CastToCharacter (Components|GetOwner)))
        (bind _asplayer_controller (Utilities|Casting|CastToPlayerController (Pawn|GetController _ascharacter)))
        (Variables|Default|SetPlayerController _asplayer_controller) ; Get PlayerController Reference
      ))))

(event EventTick
  (params (DeltaSeconds :type Float%20%28single-precision%29))
  ;[1 1 1] EVENT TICK
  (|CallParentFunction DeltaSeconds)
  (Utilities|IsLocallyControlled
    (:LocalControl
      (Networking|SwitchHasAuthority
        (:Authority
          ;;[1 1 1] Listen server?
          (if (not (Networking|IsDedicatedServer))
            ;;[1 1 1] Handle Selection
            (bind _returnvalue (Class|KJModToolProxy|GetPawnCameraComponent :!label _label))
            (bind (_outhit _returnvalue_2) (Collision|LineTraceByChannel (Transformation|GetWorldLocation _returnvalue) (+ (Transformation|GetWorldLocation _returnvalue) (* (Math|Vector|GetForwardVector _returnvalue) 3.5e+03)) "TraceTypeQuery1" false (Utilities|Array|MakeArray (Game|Player|GetPlayerPawn 0)) "None"))
            (Utilities|FlowControl|Sequence
              (:then_0
                (if _returnvalue_2
                  (if (Utilities|Struct|BreakPrecisionToolActorSettings (Variables|ToolSetting|GetSettings))
                    (bind (_isvalid _cause) (CallFunction|ActorValidforPrecisionTool (.HitActor (Collision|BreakHitResult _outhit)) (.HitComponent (Collision|BreakHitResult _outhit))))
                    (Variables|Default|SetCause _cause)
                    (if _isvalid
                      (Class|KJModUtilityActor|AddObjectHighlight (Variables|Default|GetPlayerController) (.HitActor (Collision|BreakHitResult _outhit)) "Green")
                      (elif (Utilities|Enum|Equal(Enum) (Variables|Default|GetCause) "NewEnumerator11")
                        _
                        (else
                          (Class|KJModUtilityActor|AddObjectHighlight (Variables|Default|GetPlayerController) (.HitActor (Collision|BreakHitResult _outhit)) "Red"))))
                    (Variables|Targeting|SetSelection (Utilities|Struct|MakePrecisionSelection (.ImpactPoint (Collision|BreakHitResult _outhit)) (.ImpactNormal (Collision|BreakHitResult _outhit)) (.HitActor (Collision|BreakHitResult _outhit)) (.HitComponent (Collision|BreakHitResult _outhit))))
                    (else
                      (Utilities|Struct|SetmembersinPrecisionSelection (Variables|Targeting|GetSelection) (.ImpactPoint (Utilities|Struct|BreakPrecisionSelection (Utilities|Struct|MakePrecisionSelection (.ImpactPoint (Collision|BreakHitResult _outhit)) (.ImpactNormal (Collision|BreakHitResult _outhit)) (.HitActor (Collision|BreakHitResult _outhit)) (.HitComponent (Collision|BreakHitResult _outhit))))) (.ImpactNormal (Utilities|Struct|BreakPrecisionSelection (Utilities|Struct|MakePrecisionSelection (.ImpactPoint (Collision|BreakHitResult _outhit)) (.ImpactNormal (Collision|BreakHitResult _outhit)) (.HitActor (Collision|BreakHitResult _outhit)) (.HitComponent (Collision|BreakHitResult _outhit))))))))
                  (elif (Utilities|Struct|BreakPrecisionToolActorSettings (Variables|ToolSetting|GetSettings))
                    (Variables|Default|SetCause "NewEnumerator9")
                    (Class|KJModUtilityActor|RemoveObjectHighlight (Variables|Default|GetPlayerController) (Variables|Default|GetLastHitActor)))))
              (:then_1
                (if (not (== (.HitActor (Collision|BreakHitResult _outhit)) (Variables|Default|GetLastHitActor)))
                  (if (!= (Variables|Default|GetLastHitActor) (Utilities|Struct|BreakPrecisionSelection (Variables|Targeting|GetSelection)))
                    (Class|KJModUtilityActor|RemoveObjectHighlight (Variables|Default|GetPlayerController) (Variables|Default|GetLastHitActor))
                    (Utilities|IsValid (.HitActor (Collision|BreakHitResult _outhit))
                      (:Is%20Valid
                        (Variables|Default|SetLastHitActor (.HitActor (Collision|BreakHitResult _outhit)))))))))))
        (:Remote
          (goto _label))))))

(event Custom|MC_PrecisionMovementVertex
  (params (Selection :type Precision%20Selection%20Structure) (Value :type Float%20%28single-precision%29))
  (bind (_impactnormal _hitactor) (Utilities|Struct|BreakPrecisionSelection Selection))
  ;[1 1 1] Move Object
  (Transformation|SetActorLocation _hitactor (+ (Transformation|GetActorLocation _hitactor) (* _impactnormal Value)) false true))

(event Custom|S_PrecisionMovementVertex
  (params (Selection :type Precision%20Selection%20Structure) (Value :type Float%20%28single-precision%29))
  ;[1 1 1] Move Object
  (CallFunction|MCPrecisionMovementVertex Selection Value))

(event EventToolProxyPrimaryMouseClick
  (params (pressed :type Boolean))
  (bind _cause (Variables|Default|GetCause))
  ;[1 1 1] LEFT MOUSE - Push Object
  (if pressed
    (Utilities|IsValid (Utilities|Struct|BreakPrecisionSelection (Variables|Targeting|GetSelection))
      (:Is%20Valid
        (if (Utilities|Enum|Equal(Enum) _cause "NewEnumerator7")
          (CallFunction|SPrecisionMovementVertex (Variables|Targeting|GetSelection) (* (Utilities|Struct|BreakPrecisionToolActorSettings (Variables|ToolSetting|GetSettings)) -1.0))
          (if (Utilities|Struct|BreakPrecisionToolActorSettings (Variables|ToolSetting|GetSettings))
            (Class|KJModToolProxy|PlayToolSoundEffect "ToolSpawnSound" false))
          (else
            (Class|KJModToolProxy|ShowMessage (Utilities|Select :Index _cause :NewEnumerator7 "" :NewEnumerator9 "Could not find an actor" :NewEnumerator8 "The actor is simulating physics (allow in settings)" :NewEnumerator10 "The actor is an elevator or a platform" :NewEnumerator11 "The selection is static or stationary" :NewEnumerator12 "The selection is not valid") 3.0 true "/Game/CustomContent/UGC2336045922/Assets/ErrorSign.ErrorSign")
            (if (Utilities|Struct|BreakPrecisionToolActorSettings (Variables|ToolSetting|GetSettings))
              (Class|KJModToolProxy|PlayToolSoundEffect "ToolIllegalOpSound" false))))))))

(event EventToolProxyCustomActionPressed
  (params (cookie :type Integer) (pressed :type Boolean))
  (bind _selection (Variables|Targeting|GetSelection))
  (bind _hitactor (Utilities|Struct|BreakPrecisionSelection _selection))
  ;[1 1 1] Use World Axis
  (if (== cookie 1)
    (if pressed
      (if (Utilities|Struct|BreakPrecisionToolActorSettings (Variables|ToolSetting|GetSettings))
        (Utilities|Struct|SetmembersinPrecisionToolActorSettings (Variables|ToolSetting|GetSettings) false)
        (bind _returnvalue (Game|SpawnActorfromClass "/Game/CustomContent/UGC2336045922/BP/Precision/WorldAxisBoundsActor.WorldAxisBoundsActor_C" (Math|Transform|MakeTransform (Transformation|GetActorLocation _hitactor) "0, 0, 0" "1,1,1") "Undefined" 0 0))
        (Variables|/Game/CustomContent/UGC2336045922/BP/Precision/WorldAxisBoundsActor.WorldAxisBoundsActor_C|SetSelectedActor _returnvalue _hitactor)
        (Default|SetBounds _returnvalue)
        (Variables|Default|SetWorldAxisActor _returnvalue)
        (else
          (Actor|DestroyActor (Variables|Default|GetWorldAxisActor))
          (Utilities|Struct|SetmembersinPrecisionToolActorSettings (Variables|ToolSetting|GetSettings) true))))))

(event EventToolProxySecondaryMouseClick
  (params (pressed :type Boolean))
  (bind _cause (Variables|Default|GetCause))
  ;[1 1 1] RIGHT MOUSE - Pull Object
  (if pressed
    (Utilities|IsValid (Utilities|Struct|BreakPrecisionSelection (Variables|Targeting|GetSelection))
      (:Is%20Valid
        (if (Utilities|Enum|Equal(Enum) _cause "NewEnumerator7")
          (CallFunction|SPrecisionMovementVertex (Variables|Targeting|GetSelection) (Utilities|Struct|BreakPrecisionToolActorSettings (Variables|ToolSetting|GetSettings)))
          (if (Utilities|Struct|BreakPrecisionToolActorSettings (Variables|ToolSetting|GetSettings))
            (Class|KJModToolProxy|PlayToolSoundEffect "ToolSpawnSound" false))
          (else
            (Class|KJModToolProxy|ShowMessage (Utilities|Select :Index _cause :NewEnumerator7 "" :NewEnumerator9 "Could not find an actor" :NewEnumerator8 "The actor is simulating physics (allow in settings)" :NewEnumerator10 "The actor is an elevator or a platform" :NewEnumerator11 "The selection is static or stationary" :NewEnumerator12 "The selection is not valid") 3.0 true "/Game/CustomContent/UGC2336045922/Assets/ErrorSign.ErrorSign")
            (if (Utilities|Struct|BreakPrecisionToolActorSettings (Variables|ToolSetting|GetSettings))
              (Class|KJModToolProxy|PlayToolSoundEffect "ToolIllegalOpSound" false))))))))

(event Custom|Setting_UseAudio
  (params (Use :type Boolean))
  ;[1 1 1] Settings (from widgets and onload)
  (Utilities|Struct|SetmembersinPrecisionToolActorSettings (Variables|ToolSetting|GetSettings) Use))

(event Custom|Settings_PrecisionAmount
  (params (Amount :type Float%20%28single-precision%29))
  ;[1 1 1] Settings (from widgets and onload)
  (Utilities|Struct|SetmembersinPrecisionToolActorSettings (Variables|ToolSetting|GetSettings) Amount))

(event Custom|Setting_NonFrozen
  (params (Allow :type Boolean))
  ;[1 1 1] Settings (from widgets and onload)
  (Utilities|Struct|SetmembersinPrecisionToolActorSettings (Variables|ToolSetting|GetSettings) Allow))

(event Custom|InitSettings
  ;[1 1 1] Init / Load previous settings
  (bind _returnvalue (Class|KJModToolProxy|LoadToolSettings "PrecisionToolSettings2021"))
  (Utilities|IsValid _returnvalue ; No save? use defaults
    (:Is%20Valid
      (bind _asprecision_tool_save_game_bp (Utilities|Casting|CastToPrecisionToolSaveGameBP _returnvalue))
      (Utilities|FlowControl|Sequence
        (:then_0
          ;[1 1 1] Local Initial settings
          (CallFunction|SettingsPrecisionAmount (Variables|/Game/CustomContent/UGC2336045922/BP/Precision/PrecisionToolSaveGameBP.PrecisionToolSaveGameBP_C|GetPrecisionAmount _asprecision_tool_save_game_bp)))
        (:then_1
          (CallFunction|SettingNonFrozen (Variables|/Game/CustomContent/UGC2336045922/BP/Precision/PrecisionToolSaveGameBP.PrecisionToolSaveGameBP_C|GetAllowNonFrozen _asprecision_tool_save_game_bp)))
        (:then_2
          (CallFunction|SettingUseAudio (Variables|/Game/CustomContent/UGC2336045922/BP/Precision/PrecisionToolSaveGameBP.PrecisionToolSaveGameBP_C|GetUseSound _asprecision_tool_save_game_bp)))
        (:then_3
          ;[1 1 1] Init settings server
          (Variables|ToolSetting|SetbServerSettingsInited true :!label _label))))
    (:Is%20Not%20Valid
      (goto _label))))

(fn ConstructionScript)

(fn CreateandShowToolsAssistInformation
  (Class|KJModToolProxy|ShowToolAssistUI)
  (Class|KJModToolProxy|SetToolAssistTitle "Precision" "Move actors precisly")
  (Class|KJModToolProxy|ClearToolAssistFunctions)
  (bind _returnvalue (Class|KJModToolProxy|CreateToolAssistFunction "Push object away from you"))
  (Class|KJModToolProxy|SetToolAssistFunctionPrimaryDetails _returnvalue "LeftMouse")
  (bind _returnvalue_2 (Class|KJModToolProxy|CreateToolAssistFunction "Pull actor to you"))
  (Class|KJModToolProxy|SetToolAssistFunctionPrimaryDetails _returnvalue_2 "RightMouse")
  (bind _returnvalue_3 (Class|KJModToolProxy|CreateToolAssistFunction "Move along world axis"))
  (Class|KJModToolProxy|SetToolAssistFunctionPrimaryDetails _returnvalue_3 "Key" "F"))

(fn ToolProxyGetToolSettingPanel
  (Utilities|IsValid (Variables|ToolSetting|GetToolSettingsWidget)
    (:Is%20Valid
      _)
    (:Is%20Not%20Valid
      (bind _returnvalue (UserInterface|CreateWidget "/Game/CustomContent/UGC2336045922/BP/Precision/Settings/PrecisionToolSettingsWidgetBP.PrecisionToolSettingsWidgetBP_C" (Game|GetPlayerController 0) self))
      (Default|CreatedEvent _returnvalue)
      (Variables|ToolSetting|SetToolSettingsWidget _returnvalue)))
  (return (Variables|ToolSetting|GetToolSettingsWidget)))

(fn ActorValidforPrecisionTool
  (params (Actor :type Actor%20Object%20Reference) (Component :type Primitive%20Component%20Object%20Reference))
  (LocalVariables|SetActorRef Actor)
  (LocalVariables|SetCompRef Component)
  (Utilities|IsValid (LocalVariables|GetActorRef)
    (:Is%20Valid
      (if (Actor|ActorHasTag (LocalVariables|GetActorRef) "WOLVEMOVING")
        (return false "NewEnumerator10")
        (else
          (switch Utilities|FlowControl|Switch|SwitchonEComponentMobility (Variables|/Script/Engine.SceneComponent|GetMobility (LocalVariables|GetCompRef))
            (:Static
              _)
            (:Stationary
              _)
            (:Movable
              (if (Utilities|Struct|BreakPrecisionToolActorSettings (Variables|ToolSetting|GetSettings))
                (return true "NewEnumerator7")
                (elif (Physics|IsSimulatingPhysics (LocalVariables|GetCompRef) "None")
                  (return false "NewEnumerator8")
                  (else
                    (return true "NewEnumerator7"))))))
          (return false "NewEnumerator11"))))
    (:Is%20Not%20Valid
      (return false "NewEnumerator12"))))